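; Interactable GAS loot chest, opened by interacting with its lock, that spawns a random weapon and a random item.
; The server applies an interacting effect during use, removes it on cancel or completion, then applies the open effect and spawns loot on an elliptical arc.
; A tag listener drives the cosmetics: open tag added swings the lid and drops the lock, removal reverses the lid and restores the lock.
; Availability tags block interaction.
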(event `self.ReceiveBeginPlay`
  ;[1 1 1] BeginPlay
  (`MovementComponent.SetUpdatedComponent` (`self.RotatingMovement`) (`self.SM_Forge_Chest_Top`))
  (bind (_asynctaskproxy _tag) (`AsyncTaskGameplayTagAddedRemoved.ListenForGameplayTagAddedOrRemoved` (`AbilitySystemBlueprintLibrary.GetAbilitySystemComponent` self) (`self.ListenTags`))
    (:`then`
      (set `self.ListenForTagAddRemovedTask` _asynctaskproxy)
      (set `self.LockStartingRelativeLocation` (`SceneComponent.RelativeLocation` (`self.SM_Forge_Chest_Lock`))))
    (:`OnTagAdded`
      (bind _returnvalue (== _tag (`self.OpenTag`)))
      (if _returnvalue
        (`self.OpenChest`)))
    (:`OnTagRemoved`
      (if _returnvalue
        (`self.CloseChest`)))))

(event `self.PreInteract`
  (params (InteractingActor :type "Actor Object Reference") (InteractionComponent :type "PrimitiveComponent Object Reference"))
  (bind _returnvalue (`AbilitySystemBlueprintLibrary.GetAbilitySystemComponent` self))
  ;[1 1 1] PreInteract
  (if (== InteractionComponent (`self.SM_Forge_Chest_Lock`))
    (`/Engine/EditorBlueprintResources/ActorMacros.Switch Has Authority`
      (:`Authority`
        (bind _returnvalue_2 (`AbilitySystemComponent.BP_ApplyGameplayEffectToSelf` _returnvalue "/Game/GASShooter/Characters/Hero/Abilities/GE_Interacting.GE_Interacting_C" 0.0 (`AbilitySystemComponent.MakeEffectContext` _returnvalue)))
        (set `self.GE_InteractingHandle` _returnvalue_2)))))

(event `self.PostInteract`
  (params (InteractingActor :type "Actor Object Reference") (InteractionComponent :type "PrimitiveComponent Object Reference"))
  (bind _returnvalue (`self.K2_GetActorRotation`))
  (bind _returnvalue_2 (`AbilitySystemBlueprintLibrary.GetAbilitySystemComponent` InteractingActor))
  (bind _weaponclasses (`self.WeaponClasses`))
  (bind _itemclasses (`self.ItemClasses`))
  ;[1 1 1] PostInteract
  (if (== InteractionComponent (`self.SM_Forge_Chest_Lock`))
    (`/Engine/EditorBlueprintResources/ActorMacros.Switch Has Authority`
      (:`Authority`
        (`AbilitySystemComponent.BP_ApplyGameplayEffectToTarget` _returnvalue_2 "/Game/GASShooter/Blueprints/GE_ChestOpen.GE_ChestOpen_C" (`AbilitySystemBlueprintLibrary.GetAbilitySystemComponent` self) 0.0 (`AbilitySystemComponent.MakeEffectContext` _returnvalue_2))
        (`AbilitySystemComponent.RemoveActiveGameplayEffect` (`AbilitySystemBlueprintLibrary.GetAbilitySystemComponent` self) (`self.GE_InteractingHandle`) -1)
        ;;[1 1 1] Spawn 1 item and 1 weapon out of the chest
        (`|ExecutionSequence`
          (:`then_0`
            (bind _location (`self.GetLocationToSpawnItem`))
            (`|SpawnActorFromClass` (`|GetArrayItem` _weaponclasses (`KismetMathLibrary.RandomInteger` (`KismetArrayLibrary.Array_Length` _weaponclasses))) (`KismetMathLibrary.MakeTransform` _location _returnvalue) "Undefined" "OverrideRootScale" null null))
          (:`then_1`
            (bind _location_2 (`self.GetLocationToSpawnItem`))
            (`|SpawnActorFromClass` (`|GetArrayItem` _itemclasses (`KismetMathLibrary.RandomInteger` (`KismetArrayLibrary.Array_Length` _itemclasses))) (`KismetMathLibrary.MakeTransform` _location_2 _returnvalue) "Undefined" "OverrideRootScale" null null)))))))

(event `OpenChest`
  (bind (_lockstartingrelativelocation_x _lockstartingrelativelocation_y _lockstartingrelativelocation_z) (`KismetMathLibrary.BreakVector` (`self.LockStartingRelativeLocation`)))
  ;[1 1 1] OpenChest
  (set `RotatingMovementComponent.RotationRate` (struct :`Pitch` 180.0) (`self.RotatingMovement`))
  (`ActorComponent.Activate` (`self.RotatingMovement`) true)
  (`|ExecutionSequence`
    (:`then_0`
      (`KismetSystemLibrary.Delay` (`self.ChestTopAnimationDuration`))
      (`MovementComponent.StopMovementImmediately` (`self.RotatingMovement`))
      (`ActorComponent.Deactivate` (`self.RotatingMovement`)))
    (:`then_1`
      ;;[1 1 1] Animate Lock Falling
      (bind (_direction _time) (`Timeline|LockFallOff` :!via `PlayFromStart`)
        (:`Update`
          (`SceneComponent.K2_SetRelativeLocation` (`self.SM_Forge_Chest_Lock`) (`KismetMathLibrary.MakeVector` _lockstartingrelativelocation_x _lockstartingrelativelocation_y (`KismetMathLibrary.Lerp` _lockstartingrelativelocation_z (- _lockstartingrelativelocation_z 60.0) (/ _time 0.2))) false false))
        (:`Finished`
          (`SceneComponent.SetVisibility` (`self.SM_Forge_Chest_Lock`) false true))))))

(event `CloseChest`
  ;[1 1 1] CloseChest
  (set `RotatingMovementComponent.RotationRate` (struct :`Pitch` -180.0) (`self.RotatingMovement`))
  (`ActorComponent.Activate` (`self.RotatingMovement`) true)
  (`KismetSystemLibrary.Delay` (`self.ChestTopAnimationDuration`))
  (`MovementComponent.StopMovementImmediately` (`self.RotatingMovement`))
  (`ActorComponent.Deactivate` (`self.RotatingMovement`))
  (`SceneComponent.SetVisibility` (`self.SM_Forge_Chest_Lock`) true true)
  (`SceneComponent.K2_SetRelativeLocation` (`self.SM_Forge_Chest_Lock`) (`self.LockStartingRelativeLocation`) false false))

(event `self.ReceiveEndPlay`
  (params (EndPlayReason :type "EEndPlayReason Enum" :default "Destroyed"))
  ;[1 1 1] EndPlay
  (bind _listenfortagaddremovedtask (`self.ListenForTagAddRemovedTask`)
    (:`then`
      (`AsyncTaskGameplayTagAddedRemoved.EndTask` _listenfortagaddremovedtask))
    (:`else`)))

(event `self.CancelInteraction`
  (params (InteractionComponent :type "PrimitiveComponent Object Reference"))
  ;[1 1 1] CancelInteraction - Player stops interacting (releases input early, stunned, etc).
  (if (== InteractionComponent (`self.SM_Forge_Chest_Lock`))
    (`AbilitySystemComponent.RemoveActiveGameplayEffect` (`AbilitySystemBlueprintLibrary.GetAbilitySystemComponent` self) (`self.GE_InteractingHandle`) -1)))

(fn `GetInteractionDuration`
  (params (InteractionComponent :type "PrimitiveComponent Object Reference"))
  (returns (ReturnValue :type "Float (double-precision)"))
  (if (== InteractionComponent (`self.SM_Forge_Chest_Lock`))
    (return (`self.OpenInteractionDuration`))
    (else
      (return 0.0))))

(fn `GetLocationToSpawnItem`
  (returns (Location :type "Vector Structure"))
  (locals (EllipseXRadius :type "Float (double-precision)" :default 100.0) (EllipseYRadius :type "Float (double-precision)" :default 150.0) (Degrees :type "Float (double-precision)" :default 0.0))
  (bind _output_get (set `local.Degrees` (`KismetMathLibrary.RandomFloatInRange` 90.0 270.0)))
  (return (+ (`self.K2_GetActorLocation`) (`KismetMathLibrary.MakeVector` (* (`local.EllipseXRadius`) (`KismetMathLibrary.DegCos` _output_get)) (* (`local.EllipseYRadius`) (`KismetMathLibrary.DegSin` _output_get)) 70.0))))

(fn `GetPostInteractSyncType`
  (params (InteractionComponent :type "PrimitiveComponent Object Reference"))
  (returns (bShouldSync :type Boolean) (Type :type "EAbilityTaskNetSyncType Enum"))
  (if (== InteractionComponent (`self.SM_Forge_Chest_Lock`))
    (return false "OnlyServerWait")
    (else
      (return false "OnlyServerWait"))))

(fn `GetPreInteractSyncType`
  (params (InteractionComponent :type "PrimitiveComponent Object Reference"))
  (returns (bShouldSync :type Boolean) (Type :type "EAbilityTaskNetSyncType Enum"))
  (if (== InteractionComponent (`self.SM_Forge_Chest_Lock`))
    (return true "OnlyClientWait")
    (else
      (return false "BothWait"))))

(fn `IsAvailableForInteraction`
  (params (InteractionComponent :type "PrimitiveComponent Object Reference"))
  (returns (ReturnValue :type Boolean))
  (return (and (== InteractionComponent (`self.SM_Forge_Chest_Lock`)) (not (`GameplayTagAssetInterface.HasAnyMatchingGameplayTags` (`AbilitySystemBlueprintLibrary.GetAbilitySystemComponent` self) (`self.AvailabilityTags`))))))

(fn `UserConstructionScript`
  (set `FallProtectionComponent.bClipBelow` true (`self.FallProtection`)))