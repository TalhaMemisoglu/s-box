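; LandmineBP is a landmine actor that explodes when something begins overlapping its Box component.
; The overlap spawns an explosion emitter and sound at the actor's location, destroys the Cube and Box components, then destroys the actor.
; A loop over overlapping actors runs before destruction with an empty body; the damage and debug print nodes are disconnected, so the blast deals no damage.
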(event `self.Box.OnComponentBeginOverlap`
  (params (OverlappedComponent :type "PrimitiveComponent Object Reference") (OtherActor :type "Actor Object Reference") (OtherComp :type "PrimitiveComponent Object Reference") (OtherBodyIndex :type Integer) (bFromSweep :type Boolean) (SweepResult :type "HitResult Structure (by ref)"))
  (bind _returnvalue (`self.K2_GetActorLocation`))
  (`GameplayStatics.SpawnEmitterAtLocation` "/Game/Realistic_Starter_VFX_Pack_Vol2/Particles/Explosion/P_Explosion_Big_B.P_Explosion_Big_B" _returnvalue)
  (`GameplayStatics.PlaySoundAtLocation` "/Game/Free_Sounds_Pack/wav/Explosion_Large_1-1.Explosion_Large_1-1" _returnvalue (struct) 1.0 1.0 0.0 null null null)
  (`ActorComponent.K2_DestroyComponent` (`self.Cube`))
  (`ActorComponent.K2_DestroyComponent` (`self.Box`))
  (for _array_element (`self.GetOverlappingActors` null)
    _)
  (`self.K2_DestroyActor`))

(fn `UserConstructionScript`)